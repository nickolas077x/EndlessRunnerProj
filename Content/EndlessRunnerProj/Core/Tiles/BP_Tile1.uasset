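; BP_Tile1 is a self-chaining track tile for an endless runner.
; On BeginPlay it spawns an obstacle at one of three random points with a random X offset, then dresses two child-actor blocks via SpawnBlock.
; SpawnBlock gives each block a random quarter-turn yaw and the default class, occasionally a random variant.
; When BP_BaseChar overlaps Box, the next tile spawns at LocationConnect; overlapping Box1 destroys this tile.
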(event OnComponentBeginOverlap(Box)
  (params (OverlappedComponent :type Primitive%20Component%20Object%20Reference) (OtherActor :type Actor%20Object%20Reference) (OtherComp :type Primitive%20Component%20Object%20Reference) (OtherBodyIndex :type Integer) (bFromSweep :type Boolean) (SweepResult :type Hit%20Result%20Structure%20%28by%20ref%29))
  (Utilities|Casting|CastToBP_BaseChar OtherActor)
  (Game|SpawnActorfromClass "BP_Tile1_C" (Math|Conversions|ToTransform(Vector) (Transformation|GetWorldLocation (Variables|Default|GetLocationConnect))) "Undefined" 0 0))

(event OnComponentBeginOverlap(Box1)
  (params (OverlappedComponent :type Primitive%20Component%20Object%20Reference) (OtherActor :type Actor%20Object%20Reference) (OtherComp :type Primitive%20Component%20Object%20Reference) (OtherBodyIndex :type Integer) (bFromSweep :type Boolean) (SweepResult :type Hit%20Result%20Structure%20%28by%20ref%29))
  (Utilities|Casting|CastToBP_BaseChar OtherActor)
  (Actor|DestroyActor))

(event EventBeginPlay
  (bind _returnvalue (Math|Random|RandomIntegerinRange 0 2))
  (bind _locationobstacle3 (Variables|Default|GetLocationObstacle3))
  (bind _locationobstacle1 (Variables|Default|GetLocationObstacle1))
  (bind _locationobstacle2 (Variables|Default|GetLocationObstacle2))
  (bind _newvar_0 (Variables|Backs|GetNewVar_0))
  (bind _returnvalue_2 (Utilities|Array|LastIndex _newvar_0))
  (bind _array (Utilities|Array|MakeArray _locationobstacle3 _locationobstacle2 _locationobstacle1))
  (bind _output (Utilities|Array|Get(acopy) _array _returnvalue))
  (bind _returnvalue_3 (Transformation|GetWorldLocation _output))
  (Utilities|FlowControl|Sequence
    (:then_0
      (Game|SpawnActorfromClass "/Game/EndlessRunnerProj/Core/Obstacles/BP_Obstacle.BP_Obstacle_C" (Math|Transform|MakeTransform (Math|Vector|MakeVector (+ (.x _returnvalue_3) (Math|Random|RandomFloatinRange -6e+02 6e+02)) (.y _returnvalue_3) (.z _returnvalue_3)) "0, 0, 0" "1,1,1") "Undefined" 0 0))
    (:then_1
      (CallFunction|SpawnBlock _returnvalue_2 (Variables|Default|GetBP_Tile_8x8) _newvar_0)
      (CallFunction|SpawnBlock _returnvalue_2 (Variables|Default|GetBP_Tile_8x8_2) _newvar_0))))

(event Collision|EventActorBeginOverlap
  (params (OtherActor :type Actor%20Object%20Reference)))

(event EventTick
  (params (DeltaSeconds :type Float%20%28single-precision%29)))

(fn ConstructionScript)

(fn SpawnBlock
  (params (Max :type Integer) (self2 :type Child%20Actor%20Component%20Object%20Reference) (Array :type Array%20of%20BP%20Tile%208x%208%20Class%20References))
  (if (>= (Math|Random|RandomIntegerinRange 0 10) 10)
    (Variables|Default|SetVar (Math|Random|RandomIntegerinRange 1 Max))
    (else
      (Variables|Default|SetVar 0)))
  (Transformation|AddWorldRotation self2 (Math|Rotator|MakeRotator 0.0 0.0 (* (Math|Random|RandomIntegerinRange 0 3) 9e+01)) false false)
  (ChildActorComponent|SetChildActorClass self2 (Utilities|Array|Get(acopy) Array (Variables|Default|GetVar))))